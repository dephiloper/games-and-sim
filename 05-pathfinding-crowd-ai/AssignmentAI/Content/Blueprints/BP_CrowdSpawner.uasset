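; BP_CrowdSpawner is a crowd spawner that sends BP_Crowd AI pawns across a circle centred on itself.
; On BeginPlay it loops over an index, stepping yaw in fixed increments to spawn pawns around the ring with a 180-degree rotation offset.
; Each pawn's AI controller is then told to move to a point derived from that offset rotation, intended as the opposite side, so paths converge through the middle.
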(event `self.ReceiveBeginPlay`
  (for _index (range 21)
    (bind _returnvalue (`KismetMathLibrary.MakeRotator` 0.0 0.0 (* _index 20.0)))
    (bind _returnvalue_2 (`KismetMathLibrary.ComposeRotators` _returnvalue (struct :`Yaw` 180.0)))
    (bind _returnvalue_3 (`AIBlueprintHelperLibrary.SpawnAIFromClass` "/Game/AI/Backup/BP_Crowd.BP_Crowd_C" null (+ (* (`KismetMathLibrary.Conv_RotatorToVector` _returnvalue) 500.0) (`self.K2_GetActorLocation`)) _returnvalue_2 false null))
    (bind _asbp_crowd (cast `/Game/AI/Backup/BP_Crowd` _returnvalue_3))
    (`AIController.MoveToLocation` (`AIBlueprintHelperLibrary.GetAIController` _asbp_crowd) (+ (* (`KismetMathLibrary.Conv_RotatorToVector` _returnvalue_2) 500.0) (`self.K2_GetActorLocation`)) -1.0 true true false true null true)))

(fn `UserConstructionScript`)