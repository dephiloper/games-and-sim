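; Player character Blueprint with a zoomable spring-arm camera that destroys NPCs it collides with.
; BeginPlay activates the camera, and the mouse wheel steps the spring arm length in or out through SetTargetArmLength, which clamps it to a fixed range.
; The Hit event casts the other actor to BP_NPC00 and destroys it when the cast succeeds.
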(event `self.ReceiveBeginPlay`
  (`ActorComponent.Activate` (`self.Camera`) false))

(event `Key|MouseScrollDown`
  (params (Key :type "Key Structure"))
  (:`Pressed`
    (`self.SetTargetArmLength` (+ 100.0 (`SpringArmComponent.TargetArmLength` (`self.SpringArm`))))))

(event `Key|MouseScrollUp`
  (params (Key :type "Key Structure"))
  (:`Pressed`
    (`self.SetTargetArmLength` (- (`SpringArmComponent.TargetArmLength` (`self.SpringArm`)) 100.0))))

(event `self.ReceiveHit`
  (params (MyComp :type "PrimitiveComponent Object Reference") (Other :type "Actor Object Reference") (OtherComp :type "PrimitiveComponent Object Reference") (bSelfMoved :type Boolean) (HitLocation :type "Vector Structure") (HitNormal :type "Vector Structure") (NormalImpulse :type "Vector Structure") (Hit :type "HitResult Structure (by ref)"))
  (bind _asbp_npc00 (cast `/Game/AI/Backup/BP_NPC00` Other))
  (`self.K2_DestroyActor` _asbp_npc00))

(fn `SetTargetArmLength`
  (params (NewArmLength :type "Float (double-precision)"))
  (set `SpringArmComponent.TargetArmLength` (`KismetMathLibrary.FClamp` NewArmLength 500.0 2000.0) (`self.SpringArm`)))

(fn `UserConstructionScript`)