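; BP_PlayerController is a player controller that provides click-and-hold movement of the controlled pawn toward the cursor.
; While the left mouse button is held, a gate lets Tick trace under the cursor on the Visibility channel and call SimpleMoveToLocation.
; Hits closer to the pawn than MinClickDistance are ignored.
; Logic for moving to a random TargetPoint actor is present but disconnected, so it never runs.
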(event `self.ReceiveBeginPlay`)

(event `self.ReceiveTick`
  (params (DeltaSeconds :type "Float (single-precision)"))
  (`/Engine/EditorBlueprintResources/StandardMacros.Gate` true :!label _label ; While key is pressed...
    (:`Exit`
      (`self.MoveToHitLocation` (`self.GetHitResultUnderCursorByChannel` "TraceTypeQuery1")) ; ..and move there.
    )))

(event `Key|LeftMouseButton`
  (params (Key :type "Key Structure"))
  (:`Pressed`
    (goto _label :!via `Open`))
  (:`Released`
    (goto _label :!via `Close`)))

(fn `GetRandomTargetPoint`
  (returns (TargetPoint :type "TargetPoint Object Reference"))
  (return (`|GetArrayItem` (`self.TargetPoints`) (`KismetMathLibrary.RandomIntegerInRange` 0 (- (`KismetArrayLibrary.Array_Length` (`self.TargetPoints`)) 1)))))

(fn `GoToRandomTargetPoint`
  (`AIBlueprintHelperLibrary.SimpleMoveToActor` self (`self.GetRandomTargetPoint`)))

(fn `MoveToHitLocation`
  (params (HitResult :type "HitResult Structure"))
  (bind (_bblockinghit _binitialoverlap _time _distance _location) (`GameplayStatics.BreakHitResult` HitResult))
  (if (>= (`KismetMathLibrary.VSize` (- (`self.K2_GetActorLocation` (`self.K2_GetPawn`)) _location)) (`self.MinClickDistance`))
    (`AIBlueprintHelperLibrary.SimpleMoveToLocation` self _location)))

(fn `UserConstructionScript`)