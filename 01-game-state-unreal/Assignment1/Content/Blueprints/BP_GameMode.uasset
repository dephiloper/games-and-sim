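; Game mode for a sphere-holing game that spawns spheres, tracks how many are holed and ends the game on a win.
; BeginPlay adds the HUD widget and spawns the first sphere, with the counter starting at -1.
; Each spawn waits briefly, increments the count, drops a sphere at a random elevated position, then checks for the target count.
; Reaching it flags the win, shows the game-over widget, pauses and enables the cursor.
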(event `self.ReceiveBeginPlay`
  ;[1 1 1] spawn sphere at the beginning
  (set `self.SpheresHoled` -1)
  (`self.Event SpawnNewSphere`)
  (bind _returnvalue (`|CreateWidget` "/Game/Blueprints/BP_UI.BP_UI_C"))
  (`UserWidget.AddToViewport` _returnvalue 0))

(event `Event SpawnNewSphere`
  ;[1 1 1] spawn new sphere, after 0.5 seconds at random position, increment the number of spheres holed & call event check win condition
  (`KismetSystemLibrary.Delay` 0.5)
  (bind _output_get (set `self.SpheresHoled` (`self.SpheresHoled`)))
  (`/Engine/EditorBlueprintResources/StandardMacros.IncrementInt` _output_get
    (:`  `
      (`|SpawnActorFromClass` "/Game/Blueprints/BP_Sphere.BP_Sphere_C" (`KismetMathLibrary.Conv_VectorToTransform` (`KismetMathLibrary.MakeVector` (.x (* (/ (`KismetMathLibrary.RandomUnitVector`) 2) 1000)) (.y (* (/ (`KismetMathLibrary.RandomUnitVector`) 2) 1000)) 500.0)) "Undefined" "OverrideRootScale" null null)
      (`self.Event CheckWinCondition`))))

(event `Event CheckWinCondition`
  ;[1 1 1] check if player has holed 5 spheres
  (if (== (`self.SpheresHoled`) 5)
    (set `self.PlayerHasWon` true)
    (`self.Event ShowEndScreen`)))

(event `Event ShowEndScreen`
  ;[1 1 1] shows the game over screen and pauses the game when triggered
  (bind _returnvalue (`|CreateWidget` "/Game/Blueprints/BP_GameOver.BP_GameOver_C"))
  (`UserWidget.AddToViewport` _returnvalue 0)
  (bind _returnvalue_2 (`GameplayStatics.SetGamePaused` true))
  (set `PlayerController.bShowMouseCursor` _returnvalue_2 (`GameplayStatics.GetPlayerController` 0)))

(fn `UserConstructionScript`)