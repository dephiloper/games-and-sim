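; BP_Paddle is a rotating paddle that swings out when activated and swings back at a fifth of the speed when deactivated.
; ActivationChanged sets a signed speed multiplier, which Tick integrates into a yaw offset clamped between zero and YawMaxLimit.
; Tick applies that offset, signed by Direction, as RootOffset's relative yaw on top of the world yaw captured at BeginPlay.
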(event `self.ReceiveBeginPlay`
  (set `self.InitialYaw` (.yaw (`SceneComponent.K2_GetComponentRotation` (`self.RootOffset`)))))

(event `self.ReceiveTick`
  (params (DeltaSeconds :type "Float (single-precision)"))
  (bind _output_get (set `self.Yaw` (`KismetMathLibrary.FMax` (`KismetMathLibrary.FMin` (+ (`self.Yaw`) (* DeltaSeconds (`self.RotationSpeed`) (`self.SpeedMultiplier`))) (`self.YawMaxLimit`)))))
  (`SceneComponent.K2_SetRelativeRotation` (`self.RootOffset`) (`KismetMathLibrary.MakeRotator` 0.0 0.0 (+ (`self.InitialYaw`) (* (`self.Direction`) _output_get))) false false))

(event `Event ActivationChanged`
  (params (Active :type Boolean))
  (if Active
    (set `self.SpeedMultiplier` 1.0)
    (else
      (set `self.SpeedMultiplier` -0.2))))

(fn `UserConstructionScript`)